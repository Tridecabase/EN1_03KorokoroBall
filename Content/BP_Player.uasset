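; Player actor that rolls or slides a physics-driven Sphere from Enhanced Input, registering the IMC_InGame mapping context on BeginPlay.
; IA_Move stores a normalized 2D direction, which Tick turns into a delta-scaled force along fixed world right and forward axes.
; While input is held, velocity is clamped to LimitSpeed.
; Without input, velocity is multiplied by AttenuationRate every tick, so damping depends on frame rate.
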(event `EnhancedInput|/Game/IA_Move`
  (params (ActionValue :type "Vector2D Structure") (ElapsedSeconds :type "Float (double-precision)") (TriggeredSeconds :type "Float (double-precision)") (InputAction :type "InputAction Object Reference" :default "/Game/IA_Move.IA_Move"))
  (:`Triggered`
    (set `self.InputDirection` (`KismetMathLibrary.Normal2D` ActionValue)))
  (:`Completed`
    (set `self.InputDirection` (0.0 0.0))))

(event `self.ReceiveTick`
  (params (DeltaSeconds :type "Float (single-precision)"))
  (if (> (`KismetMathLibrary.VSize2DSquared` (`self.InputDirection`)) 0.0)
    (`self.Move`)
    (`self.SetLimitSpeed`)
    (else
      (`self.Attenuation`))))

(event `self.ReceiveBeginPlay`
  (`EnhancedInputSubsystemInterface.AddMappingContext` (pcsubsystem `EnhancedInputLocalPlayerSubsystem` (`GameplayStatics.GetPlayerController` 0)) "/Game/IMC_InGame.IMC_InGame" 0 (struct)))

(fn `Attenuation`
  (bind _returnvalue (`PrimitiveComponent.GetPhysicsLinearVelocity` (`self.Sphere`) "None"))
  (`PrimitiveComponent.SetPhysicsLinearVelocity` (`self.Sphere`) (* _returnvalue (`self.AttenuationRate`)) false "None"))

(fn `Move`
  (bind (_x _y) (`KismetMathLibrary.BreakVector2D` (* (`self.InputDirection`) (* (`GameplayStatics.GetWorldDeltaSeconds`) (`self.Acceleration`)))))
  (`PrimitiveComponent.AddForce` (`self.Sphere`) (+ (* (`KismetMathLibrary.Vector_Right`) _x) (* (`KismetMathLibrary.Vector_Forward`) _y)) "None" false))

(fn `SetLimitSpeed`
  (returns (Sphere :type "StaticMeshComponent Object Reference"))
  (locals (Velocity :type "Vector Structure" :default (0.0 0.0 0.0)))
  (bind _returnvalue (`PrimitiveComponent.GetPhysicsLinearVelocity` (`self.Sphere`) "None"))
  (bind _output_get (set `local.Velocity` _returnvalue))
  (if (> (`KismetMathLibrary.VSize` _output_get) (`self.LimitSpeed`))
    (`PrimitiveComponent.SetPhysicsLinearVelocity` (`self.Sphere`) (* (`KismetMathLibrary.Normal` (`local.Velocity`)) (`self.LimitSpeed`)) false "None")))

(fn `UserConstructionScript`)