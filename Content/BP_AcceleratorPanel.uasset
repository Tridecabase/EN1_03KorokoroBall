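; BP_AcceleratorPanel is an actor that launches physics components that touch it along the panel's forward direction.
; The Cone component's begin-overlap event passes the overlapping component to the Acceleration function.
; That function snaps the component to the Cone's location, zeroes its angular velocity and replaces its linear velocity with the actor's forward vector scaled by Power, so incoming momentum is discarded.
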(event `self.Cone.OnComponentBeginOverlap`
  (params (OverlappedComponent :type "PrimitiveComponent Object Reference") (OtherActor :type "Actor Object Reference") (OtherComp :type "PrimitiveComponent Object Reference") (OtherBodyIndex :type Integer) (bFromSweep :type Boolean) (SweepResult :type "HitResult Structure (by ref)"))
  (`self.Acceleration` OtherComp))

(fn `Acceleration`
  (params (OtherComp :type "PrimitiveComponent Object Reference"))
  (`SceneComponent.K2_SetWorldLocation` OtherComp (`SceneComponent.K2_GetComponentLocation` (`self.Cone`)) false false)
  (`PrimitiveComponent.SetPhysicsAngularVelocityInRadians` (`local.OtherComp`) (0.0 0.0 0.0) false "None")
  (`PrimitiveComponent.SetPhysicsLinearVelocity` (`local.OtherComp`) (* (`self.GetActorForwardVector`) (`self.Power`)) false "None"))

(fn `UserConstructionScript`)