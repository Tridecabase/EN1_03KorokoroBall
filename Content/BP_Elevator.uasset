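; BP_Elevator is an actor that moves a Cylinder component continuously along its Spline.
; Each Tick advances a distance by SpeedSpline and DeltaSeconds, then sets the cylinder's relative transform from the spline's local location and rotation at that distance.
; The cylinder follows spline pitch and yaw with a -90 degree pitch offset, keeping its scale.
; With IsLoop enabled, the distance resets to the start after passing the spline's end.
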(event `self.ReceiveTick`
  (params (DeltaSeconds :type "Float (single-precision)"))
  (bind _returnvalue (`SplineComponent.GetTransformAtDistanceAlongSpline` (`self.Spline`) (`self.Position_spline`) "Local" false))
  (set `self.Position_spline` (+ (* DeltaSeconds (`self.Speed_spline`)) (`self.Position_spline`)))
  (`SceneComponent.K2_SetRelativeTransform` (`self.Cylinder`) (`KismetMathLibrary.MakeTransform` (.location _returnvalue) (`KismetMathLibrary.MakeRotator` 0.0 (+ (.pitch (.rotation _returnvalue)) -90.0) (.yaw (.rotation _returnvalue))) (`SceneComponent.RelativeScale3D` (`self.Cylinder`))) false false)
  (if (`self.isLoop`)
    (if (> (`self.Position_spline`) (`SplineComponent.GetSplineLength` (`self.Spline`)))
      (set `self.Position_spline` 0.0))))

(fn `UserConstructionScript`)